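; Player hero character for a twin-stick shooter, handling movement, aiming, firing, death and pausing.
; BeginPlay attaches a spawned weapon to the gunHand socket, records the spawn transform in twinStickMode and adds the HUD.
; Move axes drive world-space movement, while look axes past a deadzone set control rotation and pull the weapon trigger.
; AffectHealth handles death with a delayed GameMode respawn, then destroys weapon and character; pause input toggles the pause widget.
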(event EventBeginPlay
  (bind _mesh (Variables|Character|GetMesh))
  (Utilities|FlowControl|Sequence
    (:then_0
      (bind _returnvalue (Game|SpawnActorfromClass "/Game/blueprints/weapon.weapon_C" (Transformation|GetWorldTransform _mesh) "Undefined" 0 0))
      (bind _output_get (Variables|Default|Setweapon _returnvalue))
      (Transformation|AttachComponentToComponent _output_get _mesh "gunHand" "SnapToTarget" "SnapToTarget" "KeepWorld" true))
    (:then_1
      (bind _astwin_stick_mode (Utilities|Casting|CastTotwinStickMode (Game|GetGameMode)))
      (bind _output_get_2 (Variables|Default|Setgame%20mode _astwin_stick_mode))
      (Variables|/Game/blueprints/twinStickMode.twinStickMode_C|SetPlayerSpawnTransform _output_get_2 (Transformation|GetActorTransform)))
    (:then_2
      (bind _returnvalue_2 (UserInterface|CreateWidget "/Game/blueprints/twinStickHud.twinStickHud_C"))
      (UserInterface|Viewport|AddtoViewport _returnvalue_2 0))))

(event Collision|EventActorBeginOverlap
  (params (OtherActor :type Actor%20Object%20Reference)))

(event EventTick
  (params (DeltaSeconds :type Float%20%28single-precision%29)))

(event EventAffectHealth
  (params (delta :type Float%20%28single-precision%29))
  (Class|BaseCharacter|CalculateHealth delta)
  (if (Variables|Default|GetisDead)
    (Input|DisableInput 0)
    (Utilities|FlowControl|Delay 3.0)
    (Default|RespawnPlayer (Variables|Default|Getgame%20mode))
    (Actor|DestroyActor (Variables|Default|Getweapon))))

(event Input|ActionEvents|InputActionpause
  (params (Key :type Key%20Structure :default "None"))
  (bind _returnvalue (Game|GetPlayerController 0))
  (bind _returnvalue_2 (Game|GetPlayerController 0))
  (:Pressed
    (if (Variables|Default|GetisPaused)
      (bind _foundwidgets (Widget|GetAllWidgetsOfClass "/Game/blueprints/pauseHud.pauseHud_C" false))
      (for _array_element _foundwidgets
        (Widget|RemovefromParent _array_element)
        (Variables|/Script/Engine.PlayerController|SetbShowMouseCursor _returnvalue false)
        (Input|SetInputModeGameOnly _returnvalue)
        (Game|SetGamePaused false)
        (Variables|Default|SetisPaused false))
      (else
        (bind _returnvalue_3 (UserInterface|CreateWidget "/Game/blueprints/pauseHud.pauseHud_C"))
        (UserInterface|Viewport|AddtoViewport _returnvalue_3 0)
        (Input|SetInputModeGameandUI _returnvalue_2 0 "DoNotLock" true)
        (Variables|/Script/Engine.PlayerController|SetbShowMouseCursor _returnvalue_2 true)
        (Variables|Default|SetisPaused true)
        (Game|SetGamePaused true)))))

(event Input|AxisEvents|InputAxismoveUp
  (params (AxisValue :type Float%20%28single-precision%29))
  ;[1 1 1] movement
  (Pawn|Input|AddMovementInput "1.000000,0.000000, 0" AxisValue false))

(event Input|AxisEvents|InputAxismoveRight
  (params (AxisValue :type Float%20%28single-precision%29))
  ;[1 1 1] movement
  (Pawn|Input|AddMovementInput "0.000000,1.000000, 0" AxisValue false))

(event Input|AxisEvents|InputAxislookUp
  (params (AxisValue :type Float%20%28single-precision%29))
  (bind _weapon (Variables|Default|Getweapon))
  ;[1 1 1] rotation
  (if (> (Math|Vector|VectorLength (Math|Vector|MakeVector AxisValue (stale Input|AxisEvents|InputAxislookRight AxisValue) 0.0)) 0.25)
    (Pawn|SetControlRotation (Pawn|GetController) (Math|Conversions|RotationFromXVector (Math|Vector|MakeVector AxisValue (stale Input|AxisEvents|InputAxislookRight AxisValue) 0.0)))
    (Default|PullTrig _weapon)
    (else
      (Default|ReleaseTrip _weapon))))

(event Input|AxisEvents|InputAxislookRight
  (params (AxisValue :type Float%20%28single-precision%29))
  (bind _weapon (Variables|Default|Getweapon))
  ;[1 1 1] rotation
  (if (> (Math|Vector|VectorLength (Math|Vector|MakeVector (stale Input|AxisEvents|InputAxislookUp AxisValue) AxisValue 0.0)) 0.25)
    (Pawn|SetControlRotation (Pawn|GetController) (Math|Conversions|RotationFromXVector (Math|Vector|MakeVector (stale Input|AxisEvents|InputAxislookUp AxisValue) AxisValue 0.0)))
    (Default|PullTrig _weapon)
    (else
      (Default|ReleaseTrip _weapon))))

(fn ConstructionScript)