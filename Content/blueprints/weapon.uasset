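; Weapon actor that fires projectiles automatically while its trigger is held.
; Pulling the trigger passes a DoOnce gate, fires immediately and starts a looping timer paced by RoundsPerSecond.
; Each shot spawns the Projectile class at the ProjectileSpawnPoint transform.
; Releasing the trigger clears the timer and resets the gate.
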(event Custom|pullTrig
  (Utilities|FlowControl|DoOnce false
    (:Completed
      (CallFunction|Fire)
      (Utilities|Time|SetTimerbyFunctionName 0 "fire" (/ 1.0 (Variables|Default|GetroundsPerSecond)) true))))

(event Custom|releaseTrip
  (Utilities|Time|ClearTimerbyFunctionName 0 "fire")
  (Utilities|FlowControl|DoOnce false) ; enters at Reset
)

(event Custom|fire
  (Game|SpawnActorfromClass "/Game/blueprints/projectile.projectile_C" (Transformation|GetWorldTransform (Variables|Default|GetprojectileSpawnPoint)) "Undefined" 0 0))

(event EventBeginPlay)

(event Collision|EventActorBeginOverlap
  (params (OtherActor :type Actor%20Object%20Reference)))

(event EventTick
  (params (DeltaSeconds :type Float%20%28single-precision%29)))

(fn ConstructionScript)