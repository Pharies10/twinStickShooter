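; Enemy character for a twin-stick game that damages the hero on contact and awards score when it dies.
; Overlapping the hero starts a looping timer that applies damage at the attack rate, cleared when the overlap ends.
; On death it increments the game mode's score, ignores pawn and world-dynamic collision, detaches its controller and is destroyed after a delay.
; The construction script tints the body through a dynamic material instance.
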(event Custom|DamageTheHero
  ;[1 1 1] Damaging hero char
  (Default|AffectHealth (Variables|Default|Gethero) (Variables|Default|GetDamage)))

(event EventBeginPlay)

(event Collision|EventActorBeginOverlap
  (params (OtherActor :type Actor%20Object%20Reference))
  ;[1 1 1] Damaging hero char
  (bind _ashero_char (Utilities|Casting|CastToheroChar OtherActor))
  (Variables|Default|Sethero _ashero_char)
  (Utilities|Time|SetTimerbyFunctionName 0 "DamageTheHero" (/ 1.0 (Variables|Default|GetattacksPerSecond)) true))

(event EventTick
  (params (DeltaSeconds :type Float%20%28single-precision%29)))

(event EventAffectHealth
  (params (delta :type Float%20%28single-precision%29))
  (bind _capsulecomponent (Variables|Default|GetCapsuleComponent))
  ;[1 1 1] Getting damaged
  (Class|BaseCharacter|CalculateHealth delta)
  (if (Variables|Default|GetisDead)
    (bind _astwin_stick_mode (Utilities|Casting|CastTotwinStickMode (Game|GetGameMode)))
    (Default|IncrementScore _astwin_stick_mode 1)
    (Collision|SetCollisionResponsetoChannel _capsulecomponent "ECC_WorldDynamic" "ECR_Ignore")
    (Collision|SetCollisionResponsetoChannel _capsulecomponent "ECC_Pawn" "ECR_Ignore")
    (Class|Pawn|DetachfromControllerPendingDestroy)
    (Utilities|FlowControl|Delay 3.0)
    (Actor|DestroyActor)))

(event Collision|EventActorEndOverlap
  (params (OtherActor :type Actor%20Object%20Reference))
  ;[1 1 1] Damaging hero char
  (if (== OtherActor (Variables|Default|Gethero))
    (Utilities|Time|ClearTimerbyFunctionName 0 "DamageTheHero")))

(fn ConstructionScript
  (bind _returnvalue (Rendering|Material|CreateDynamicMaterialInstance (Variables|Character|GetMesh) 0 0 "None" :!class /Script/Engine.PrimitiveComponent))
  (bind _output_get (Variables|Default|SetdynMat _returnvalue))
  (Rendering|Material|SetVectorParameterValue _output_get "BodyColor" (Variables|Default|GetenemyColor) :!class /Script/Engine.MaterialInstanceDynamic))